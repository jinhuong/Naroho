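; BP_Rocket is an actor that flies a cone mesh along a spline as a rocket.
; Each Tick it grows a travelled distance by speed times delta time, then samples the spline's local-space transform at that distance.
; The cone takes that location and rotation, with pitch offset by -90 degrees, presumably to point its tip along the path.
; The file contains no looping, end-of-path or collision logic.
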(event `self.ReceiveTick`
  (params (DeltaSeconds :type "Float (single-precision)"))
  (bind _returnvalue (`SplineComponent.GetTransformAtDistanceAlongSpline` (`self.Spline`) (`self.Rocket_Distance`) "Local" false))
  (set `self.Rocket_Distance` (+ (* (`GameplayStatics.GetWorldDeltaSeconds`) (`self.Rocket_Speed`)) (`self.Rocket_Distance`)))
  (`SceneComponent.K2_SetRelativeTransform` (`self.Cone`) (`KismetMathLibrary.MakeTransform` (.location _returnvalue) (`KismetMathLibrary.MakeRotator` (.roll (.rotation _returnvalue)) (+ (.pitch (.rotation _returnvalue)) -90.0) (.yaw (.rotation _returnvalue)))) false false))

(fn `UserConstructionScript`)