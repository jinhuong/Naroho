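; BP_Naroho is an actor that moves its Cone component along its Spline.
; Each Tick adds Speed times world delta seconds to an accumulated Distance, then samples the spline's local-space location and rotation at that distance.
; The sampled values become the cone's relative transform; Distance has no wrap or clamp.
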(event `self.ReceiveTick`
  (params (DeltaSeconds :type "Float (single-precision)"))
  (bind (_returnvalue_location _returnvalue_rotation) (`KismetMathLibrary.BreakTransform` (`SplineComponent.GetTransformAtDistanceAlongSpline` (`self.Spline`) (`self.Distance`) "Local" false)))
  (set `self.Distance` (+ (* (`GameplayStatics.GetWorldDeltaSeconds`) (`self.Speed`)) (`self.Distance`)))
  (`SceneComponent.K2_SetRelativeTransform` (`self.Cone`) (`KismetMathLibrary.MakeTransform` _returnvalue_location _returnvalue_rotation) false false))

(fn `UserConstructionScript`)