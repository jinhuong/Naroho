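; Rocket actor that attaches a particle system on BeginPlay and lifts off along its up vector after a timed wait.
; Tick accumulates elapsed time, starts movement once it passes both DelayTime and a fixed threshold, then raises Speed above a height threshold.
; Independently of launch timing, it plays a radial world camera shake at its location every tick until it climbs past a height limit.
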(event `self.ReceiveBeginPlay`
  (`AddComponent|NODE_AddParticleSystemComponent-0` :`RelativeTransform` (`KismetMathLibrary.MakeTransform` (0.0 0.0 0.0) (struct :`Pitch` 180.0))))

(event `self.ReceiveTick`
  (params (DeltaSeconds :type "Float (single-precision)"))
  (bind (_returnvalue_x _returnvalue_y _returnvalue_z) (`KismetMathLibrary.BreakVector` (`self.K2_GetActorLocation`)))
  (bind (_returnvalue_x_2 _returnvalue_y_2 _returnvalue_z_2) (`KismetMathLibrary.BreakVector` (`self.K2_GetActorLocation`)))
  (bind (_returnvalue_x_3 _returnvalue_y_3 _returnvalue_z_3) (`KismetMathLibrary.BreakVector` (`self.K2_GetActorLocation`)))
  (`|ExecutionSequence`
    (:`then_0`
      (bind _output_get (set `self.CurentTime` (+ (`GameplayStatics.GetWorldDeltaSeconds`) (`self.CurentTime`))))
      (if (> _output_get (`self.DelayTime`))
        (if (> (`self.CurentTime`) 8.0)
          (`self.K2_SetActorLocation` (+ (`self.K2_GetActorLocation`) (* (* (`self.GetActorUpVector`) (`self.Speed`)) (`GameplayStatics.GetWorldDeltaSeconds`))))
          (if (> _returnvalue_z_2 2000.0)
            (set `self.Speed` 5000.0)
            (if (> _returnvalue_z 2500.0)
              _)))))
    (:`then_1`
      (if (> 3000.0 _returnvalue_z_3)
        (`self.CameraShake`)))))

(event `CameraShake`
  (`GameplayStatics.PlayWorldCameraShake` "/Game/Jin/BluePrint/BP_Main/BP_LegacyCamerashake.BP_LegacyCamerashake_C" (`self.K2_GetActorLocation`) 30.0 500.0))

(fn `UserConstructionScript`)